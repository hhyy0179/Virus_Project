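; BP_VirusHUD is a HUD Blueprint that draws a red target crosshair texture on screen.
; Each DrawHUD call finds the screen center, raises that point by a fixed offset, and subtracts half-size variables to position the fixed-size texture.
; BeginPlay, Tick, overlap and the construction script are empty.
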(event EventBeginPlay)

(event Collision|EventActorBeginOverlap
  (params (OtherActor :type Actor%20Object%20Reference)))

(event EventTick
  (params (DeltaSeconds :type Float%20%28single-precision%29)))

(event EventDrawHUD
  (params (SizeX :type Integer) (SizeY :type Integer))
  (Variables|Default|SetScreen%20Center (Math|Vector2D|MakeVector2D (Math|Conversions|ToFloat(Integer) (/ SizeX 2)) (Math|Conversions|ToFloat(Integer) (/ SizeY 2))))
  (Variables|Default|SetTargetLocation (Math|Vector2D|MakeVector2D (.X (Math|Vector2D|BreakVector2D (Variables|Default|GetScreen%20Center))) (- (.Y (Math|Vector2D|BreakVector2D (Variables|Default|GetScreen%20Center))) 5e+01)))
  (Canvas|DrawTexture "/Game/_VirusGame/ScanFX/Image/target2_red.target2_red" (- (.X (Math|Vector2D|BreakVector2D (Variables|Default|GetTargetLocation))) (Variables|Default|GetTargetHalfWidth)) (- (.Y (Math|Vector2D|BreakVector2D (Variables|Default|GetTargetLocation))) (Variables|Default|GetTargetHalfHeight)) 4e+01 4e+01 0.0 0.0 1.0 1.0 "(R=1.000000,G=1.000000,B=1.000000,A=1.000000)"))

(fn ConstructionScript)