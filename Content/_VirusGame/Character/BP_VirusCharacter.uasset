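; BP_VirusCharacter is a character Blueprint for the virus game, holding health and movement-speed logic.
; Pressing Left Shift directly subtracts a fixed amount from CurrentHP, with no clamp or death check in this graph.
; Two CCTV-related events drive walk speed: decrease scales the current max speed down, so repeated calls compound, while increase sets a fixed value.
; BeginPlay, overlap, Tick and the construction script are empty.
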(event Custom|Increase_Speed_Event
  ;[1 1 1] CCTV 이동속도
  (Variables|/Script/Engine.CharacterMovementComponent|SetMaxWalkSpeed (Variables|Character|GetCharacterMovement) 3e+02))

(event Custom|Decrease_Speed_Event
  (bind _charactermovement (Variables|Character|GetCharacterMovement))
  ;[1 1 1] CCTV 이동속도
  (Variables|/Script/Engine.CharacterMovementComponent|SetMaxWalkSpeed _charactermovement (* (Class|MovementComponent|GetMaxSpeed _charactermovement) 0.7)))

(event EventBeginPlay)

(event Collision|EventActorBeginOverlap
  (params (OtherActor :type Actor%20Object%20Reference)))

(event EventTick
  (params (DeltaSeconds :type Float%20%28single-precision%29)))

(event Input|KeyboardEvents|LeftShift
  (params (Key :type Key%20Structure))
  ;[1 1 1] 체력
  (:Pressed
    (Variables|Default|SetCurrentHP (- (Variables|Default|GetCurrentHP) 1e+01))))

(fn ConstructionScript)