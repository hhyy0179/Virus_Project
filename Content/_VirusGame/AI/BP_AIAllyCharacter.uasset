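; BP_AIAllyCharacter is an ally AI character that follows program characters it sees.
; PawnSensing stores a sighted BP_AIProgramCharacter and, if it is over 100 units away, flags it as seen and runs FollowActor.
; FollowActor issues an AIMoveTo toward that character, while closer sightings only print a debug message.
; The overlap handler looks unfinished: it calls GetCurrentHP on an overlapping program character but ignores the result.
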(event OnSeePawn(PawnSensing)
  (params (Pawn :type Pawn%20Object%20Reference))
  (bind _asbp_aiprogram_character (Utilities|Casting|CastToBP_AIProgramCharacter Pawn))
  (Variables|Default|SetAIProgram _asbp_aiprogram_character)
  (if (<= (Math|Vector|VectorLength (- (Transformation|GetActorLocation Pawn) (Transformation|GetActorLocation))) 1e+02)
    (Development|PrintString "close")
    (else
      (Variables|Default|SetIsSeeingPawn true)
      (CallFunction|FollowActor))))

(event Custom|Follow%20Actor
  (AI|AIMoveTo self "0, 0, 0" (Variables|Default|GetAIProgram) 5.0 false
    (:OnFail
      (Development|PrintText "fail"))))

(event Collision|EventActorBeginOverlap
  (params (OtherActor :type Actor%20Object%20Reference))
  (Development|PrintString "overlap begin")
  (bind _asbp_aiprogram_character (Utilities|Casting|CastToBP_AIProgramCharacter OtherActor))
  (Class|AIProgramCharacter|GetCurrentHP _asbp_aiprogram_character))

(event EventBeginPlay
  (Development|PrintString "Hello"))

(fn ConstructionScript)