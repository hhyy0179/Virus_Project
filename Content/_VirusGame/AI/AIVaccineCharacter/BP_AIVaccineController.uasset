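; AI controller for the vaccine enemy that perceives and attacks the player's virus character.
; On possess it caches the vaccine character and runs BT_AIVaccine, while perception updates store the virus character and set the CanSeePlayer blackboard key.
; Walk and Run events forward to the pawn.
; Attack triggers the pawn's attack, subtracts fixed damage directly from the player's HP, then clears CanSeePlayer.
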(event OnTargetPerceptionUpdated(AIPerception)
  (params (Actor :type Actor%20Object%20Reference) (Stimulus :type AI%20Stimulus%20Structure))
  (bind _asbp_virus_character (Utilities|Casting|CastToBP_VirusCharacter Actor))
  (Variables|Default|SetPlayerCharacter _asbp_virus_character)
  (AI|Components|Blackboard|SetValueasBool (AI|GetBlackboard 0) (Utilities|Name|MakeLiteralName "CanSeePlayer") (.bSuccessfullySensed (Utilities|Struct|BreakAIStimulus Stimulus))))

(event Custom|Walk
  (Default|Walk (Variables|Default|GetVaccineCharacter)))

(event Custom|Run
  (Default|Run (Variables|Default|GetVaccineCharacter)))

(event Custom|Attack
  (bind _playercharacter (Variables|Default|GetPlayerCharacter))
  (Default|Attack (Variables|Default|GetVaccineCharacter))
  (Variables|/Script/Virus.VirusCharacter|SetCurrentHP _playercharacter (- (Variables|/Script/Virus.VirusCharacter|GetCurrentHP _playercharacter) 15.0))
  (AI|Components|Blackboard|SetValueasBool (AI|GetBlackboard 0) (Utilities|Name|MakeLiteralName "CanSeePlayer") false))

(event EventPossess
  (params (PossessedPawn :type Pawn%20Object%20Reference))
  (bind _asbp_aivaccine_character (Utilities|Casting|CastToBP_AIVaccineCharacter PossessedPawn))
  (Variables|Default|SetVaccineCharacter _asbp_aivaccine_character)
  (AI|RunBehaviorTree "/Game/_VirusGame/AI/AIVaccineCharacter/BT_AIVaccine.BT_AIVaccine"))

(fn ConstructionScript)