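; BP_AIVaccineCharacter is the AI vaccine character, with walk and run speed switching and a needle attack.
; Attack plays the AM_AIVaccine montage's Attack section and drops to walk speed.
; After a short delay it attaches a SpawnEmitterActor to the Niddle socket, plays a 2D sound and destroys the emitter immediately.
; Hit is an empty stub, and an older Stabbing animation chain is left unconnected.
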(event Custom|Walk
  (Variables|/Script/Engine.CharacterMovementComponent|SetMaxWalkSpeed (Variables|Character|GetCharacterMovement) 1.5e+02))

(event Custom|Run
  (Variables|/Script/Engine.CharacterMovementComponent|SetMaxWalkSpeed (Variables|Character|GetCharacterMovement) 2e+02))

(event Custom|Attack
  (bind _mesh (Variables|Character|GetMesh))
  (bind _returnvalue (Components|SkeletalMesh|GetAnimInstance _mesh))
  (Animation|Montage|MontagePlay _returnvalue "/Game/_VirusGame/AI/AIVaccineCharacter/Anim/AM_AIVaccine.AM_AIVaccine" 1.3 "MontageLength" 0.0 true)
  (Ability|Animation|MontageJumptoSection _returnvalue "Attack" "/Game/_VirusGame/AI/AIVaccineCharacter/Anim/AM_AIVaccine.AM_AIVaccine")
  (CallFunction|Walk)
  (Utilities|FlowControl|Delay 0.5)
  (bind _returnvalue_2 (Game|SpawnActorfromClass "/Game/_VirusGame/AI/SpawnEmitterActor.SpawnEmitterActor_C" (Math|Conversions|ToTransform(Vector) "0, 0, 0") "Undefined" 0 0))
  (Transformation|AttachComponentToComponent _returnvalue_2 (Variables|Character|GetMesh) "Niddle" "KeepRelative" "KeepRelative" "KeepRelative" true)
  (Audio|PlaySound2D "/Game/_VirusGame/Sound/340335__smullen93__attacksound_boxer_tsss03.340335__smullen93__attacksound_boxer_tsss03" 1.0 1.0 0.0 0 0)
  (Actor|DestroyActor _returnvalue_2))

(event EventBeginPlay
  (Variables|/Script/Engine.CharacterMovementComponent|SetMaxWalkSpeed (Variables|Character|GetCharacterMovement) 1.5e+02))

(event Collision|EventHit
  (params (MyComp :type Primitive%20Component%20Object%20Reference) (Other :type Actor%20Object%20Reference) (OtherComp :type Primitive%20Component%20Object%20Reference) (bSelfMoved :type Boolean) (HitLocation :type Vector :default "0, 0, 0") (HitNormal :type Vector :default "0, 0, 0") (NormalImpulse :type Vector :default "0, 0, 0") (Hit :type Hit%20Result%20Structure%20%28by%20ref%29)))

(fn ConstructionScript)