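; AI ally character Blueprint that walks at a fixed slow speed and provides an Attack event.
; Attack overrides the mesh with a one-shot zombie attack animation, then briefly waits to spawn an emitter actor attached to the mesh's emitter socket.
; A second fixed delay hands the mesh back to its Animation Blueprint, so timing relies on delays rather than anim notifies.
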(event Custom|Attack
  (bind _mesh (Variables|Character|GetMesh))
  (Components|Animation|PlayAnimation _mesh "/Game/_VirusGame/AI/AIAllyCharacter/Anim_AIAlly/NewWalking/Zombie_Attack.Zombie_Attack" false)
  (Utilities|FlowControl|Delay 0.2)
  (bind _returnvalue (Game|SpawnActorfromClass "/Game/_VirusGame/AI/AIAllyCharacter/SpawnEmitterActor.SpawnEmitterActor_C" (Math|Conversions|ToTransform(Vector) "0, 0, 0") "Undefined" 0 0))
  (Transformation|AttachComponentToComponent _returnvalue (Variables|Character|GetMesh) "EmitterSpawnSocket" "KeepRelative" "KeepRelative" "KeepRelative" true)
  (Utilities|FlowControl|Delay 1.8)
  (Components|Animation|SetAnimationMode _mesh "AnimationBlueprint"))

(event EventBeginPlay
  (Variables|/Script/Engine.CharacterMovementComponent|SetMaxWalkSpeed (Variables|Character|GetCharacterMovement) 1.5e+02))

(fn ConstructionScript)