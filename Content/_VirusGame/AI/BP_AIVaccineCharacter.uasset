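; AI enemy character, a vaccine, that chases and attacks the player's virus character.
; PawnSensing starts an AI MoveTo chase with a looping walk animation when it sees a distant player, and plays a stab animation, gated by a one-second delay, at close range.
; Damage is separate from the stab: any actor overlap with a VirusCharacter subtracts a fixed amount of HP and prints debug output.
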(event OnSeePawn(PawnSensing_0)
  (params (Pawn :type Pawn%20Object%20Reference))
  (if (Pawn|IsPlayerControlled Pawn)
    (if (<= (Math|Vector|VectorLength (- (Transformation|GetActorLocation Pawn) (Transformation|GetActorLocation))) 1e+02)
      (if (not (Variables|Default|GetisAnimationPlay))
        (Variables|Default|SetisAnimationPlay true)
        (Components|Animation|PlayAnimation (Variables|Character|GetMesh) "/Game/_VirusGame/AI/TempAnim/Stabbing.Stabbing" false)
        (Utilities|FlowControl|Delay 1.0)
        (Variables|Default|SetisAnimationPlay false))
      (else
        (Variables|Default|SetisSeeingPawn_0 true)
        (CallFunction|FollowPlayer)))))

(event Custom|FollowPlayer
  (if (Variables|Default|GetisSeeingPawn_0)
    (AI|AIMoveTo self "0, 0, 0" (Game|GetPlayerCharacter 0) 5.0 false
      (:then
        (Components|Animation|PlayAnimation (Variables|Character|GetMesh) "/Game/_VirusGame/AI/TempAnim/Walking__1_.Walking__1_" true)))))

(event EventBeginPlay)

(event Collision|EventActorBeginOverlap
  (params (OtherActor :type Actor%20Object%20Reference))
  (Development|PrintString "overlap begin")
  (bind _asvirus_character (Utilities|Casting|CastToVirusCharacter OtherActor))
  (bind _returnvalue (Class|VirusCharacter|GetHP _asvirus_character))
  (bind _output_get (Variables|/Script/Virus.VirusCharacter|SetCurrentHP _asvirus_character (- _returnvalue 1e+01)))
  (Development|PrintString (Utilities|String|ToString(Float) _output_get)))

(fn ConstructionScript)