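; Brain boss actor that fires moving lasers and ends the game with a clear when it dies.
; On BeginPlay it adds the boss HP widget and starts a self-repeating loop that spawns lasers at a fixed offset after random delays.
; Tick spins the mesh and two rings at different rates.
; Die resets the hacking gauge to a small value and calls GameClear on the UI manager.
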(event Custom|SpawnLaser
  (bind _returnvalue (Transformation|GetActorTransform))
  (Game|SpawnActorfromClass "/Game/_VirusGame/AI/AIOperatingSystem/BP_MovingLaser.BP_MovingLaser_C" (Math|Transform|MakeTransform (Math|Vector|MakeVector (+ (.x (.location _returnvalue)) 1e+03) (+ (.y (.location _returnvalue)) 9.2e+02) (- (.z (.location _returnvalue)) 5.3e+02)) (Variables|Default|GetBrainRotation) (.scale _returnvalue)) "AlwaysSpawn" 0 0)
  (Utilities|FlowControl|Delay (* (Math|Random|RandomFloat) 4.0))
  (CallFunction|SpawnLaser))

(event Custom|Die
  (bind _returnvalue (Actor|GetActorOfClass "/Script/Virus.HackingGaugeManager"))
  (Variables|/Script/Virus.HackingGaugeManager|SetPercent _returnvalue 0.0)
  (Class|HackingGaugeManager|ControlGauge _returnvalue (+ (Variables|/Script/Virus.HackingGaugeManager|GetPercent _returnvalue) 0.2))
  (bind _returnvalue_2 (Actor|GetActorOfClass "/Game/_VirusGame/Actor/BP_UIManager.BP_UIManager_C"))
  (Default|GameClear _returnvalue_2))

(event EventBeginPlay
  (Variables|Default|SetBrainRotation (Transformation|GetActorRotation))
  (CallFunction|SpawnLaser)
  (bind _returnvalue (UserInterface|CreateWidget "/Game/_VirusGame/HUD/BP_BossHP.BP_BossHP_C"))
  (UserInterface|Viewport|AddtoViewport _returnvalue 0))

(event EventTick
  (params (DeltaSeconds :type Float%20%28single-precision%29))
  (Transformation|AddWorldRotation (Variables|Default|GetStaticMesh) "0.000000,0.500000,0.000000" false false)
  (Transformation|AddWorldRotation (Variables|Default|GetCircle1) "0.000000,1.000000,0.000000" false false)
  (Transformation|AddWorldRotation (Variables|Default|GetCircle2) "0.000000,-0.600000,0.000000" false false))

(fn ConstructionScript)