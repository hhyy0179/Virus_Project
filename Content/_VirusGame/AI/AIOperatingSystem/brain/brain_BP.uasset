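; Brain actor in the AI operating system area that spins constantly and repeatedly spawns moving lasers.
; BeginPlay caches the starting rotation and starts SpawnLaser, which re-triggers itself after a random delay of up to a few seconds.
; Each BP_MovingLaser appears at a fixed world-space offset from the brain with that cached rotation, so the per-frame spin, which is not delta-time scaled, does not affect laser orientation.
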(event Custom|SpawnLaser
  (bind _returnvalue (Transformation|GetActorTransform))
  (Game|SpawnActorfromClass "/Game/_VirusGame/AI/AIOperatingSystem/BP_MovingLaser.BP_MovingLaser_C" (Math|Transform|MakeTransform (Math|Vector|MakeVector (+ (.x (.location _returnvalue)) 1e+03) (+ (.y (.location _returnvalue)) 9.2e+02) (- (.z (.location _returnvalue)) 5.3e+02)) (Variables|Default|GetBrainRotation) (.scale _returnvalue)) "AlwaysSpawn" 0 0)
  (Utilities|FlowControl|Delay (* (Math|Random|RandomFloat) 4.0))
  (CallFunction|SpawnLaser))

(event EventBeginPlay
  (Variables|Default|SetBrainRotation (Transformation|GetActorRotation))
  (CallFunction|SpawnLaser))

(event EventTick
  (params (DeltaSeconds :type Float%20%28single-precision%29))
  (Class|Actor|AddActorWorldRotation "0.000000,0.500000,0.000000"))

(fn ConstructionScript)