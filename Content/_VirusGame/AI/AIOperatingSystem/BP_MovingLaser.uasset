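; BP_MovingLaser is a laser actor in the AI Operating System folder that travels in a straight line for a limited lifetime.
; BeginPlay disables collision on its NiagaraLaser component, then destroys the actor after a 20-second delay.
; Tick moves it along world +X by a fixed step each frame without sweep, so speed depends on frame rate.
; The graph contains no active overlap or damage logic.
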(event EventBeginPlay
  (bind _niagaralaser (Variables|Default|GetNiagaraLaser))
  (|CallParentFunction)
  (Collision|SetCollisionResponsetoAllChannels _niagaralaser "ECR_Ignore")
  (Collision|SetCollisionEnabled _niagaralaser "NoCollision")
  (Utilities|FlowControl|Delay 2e+01)
  (Actor|DestroyActor))

(event Collision|EventActorBeginOverlap
  (params (OtherActor :type Actor%20Object%20Reference))
  (|CallParentFunction OtherActor) ; This node is disabled and will not be called.\nDrag off pins to build functionality.
)

(event EventTick
  (params (DeltaSeconds :type Float%20%28single-precision%29))
  (|CallParentFunction DeltaSeconds)
  (Transformation|SetActorLocation (+ (Transformation|GetActorLocation) "5.000000,0.000000,0.000000") false false))

(fn ConstructionScript
  (|CallParentFunction))