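; BP_UIManager is an actor that owns the player HUD and the end-of-game screens.
; On BeginPlay it creates BP_CharacterUI and adds it to the viewport, then forwards Q and E cooldown and lock-icon removal events to that widget.
; GameClear and GameOver each show their own screen widget, wait a short delay, then open the Main level.
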(event Custom|GameClear
  (bind _returnvalue (UserInterface|CreateWidget "/Game/_VirusGame/HUD/BP_GameClearScreen.BP_GameClearScreen_C"))
  (UserInterface|Viewport|AddtoViewport _returnvalue 0)
  (Utilities|FlowControl|Delay 5.0)
  (Game|OpenLevel(byObjectReference) "/Game/_VirusGame/Maps/Main.Main"))

(event Custom|GameOver
  (bind _returnvalue (UserInterface|CreateWidget "/Game/_VirusGame/HUD/BP_GameOverScreen.BP_GameOverScreen_C"))
  (UserInterface|Viewport|AddtoViewport _returnvalue 0)
  (Utilities|FlowControl|Delay 5.0)
  (Game|OpenLevel(byObjectReference) "/Game/_VirusGame/Maps/Main.Main"))

(event Custom|Q_Cooldown
  (Default|QCooldown (stale EventBeginPlay _returnvalue)))

(event Custom|E_Cooldown
  (Default|ECooldown (stale EventBeginPlay _returnvalue)))

(event Custom|DeleteLockIcon
  (Default|DeleteLockIcon (stale EventBeginPlay _returnvalue)))

(event EventBeginPlay
  (bind _returnvalue (UserInterface|CreateWidget "/Game/_VirusGame/HUD/BP_CharacterUI.BP_CharacterUI_C"))
  (UserInterface|Viewport|AddtoViewport _returnvalue 0))

(fn ConstructionScript)