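; BP_BossPortal is a trigger actor that sends the virus player into the boss encounter.
; When a BP_VirusCharacter overlaps its Box, it moves the character to the first TargetPoint found in the level and adds the BP_BossHP widget to the viewport.
; It then spawns the Brain_BP boss at a hardcoded transform, with no guard against repeat triggers.
; Other overlapping actors only print a debug string.
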(event OnComponentBeginOverlap(Box)
  (params (OverlappedComponent :type Primitive%20Component%20Object%20Reference) (OtherActor :type Actor%20Object%20Reference) (OtherComp :type Primitive%20Component%20Object%20Reference) (OtherBodyIndex :type Integer) (bFromSweep :type Boolean) (SweepResult :type Hit%20Result%20Structure%20%28by%20ref%29))
  (bind _asbp_virus_character (Utilities|Casting|CastToBP_VirusCharacter OtherActor)
    (:then
      (bind _outactors (Actor|GetAllActorsOfClass "/Script/Engine.TargetPoint"))
      (Transformation|SetActorLocation _asbp_virus_character (Transformation|GetActorLocation (Utilities|Array|Get(acopy) _outactors)) false false)
      (bind _returnvalue (UserInterface|CreateWidget "/Game/_VirusGame/HUD/BP_BossHP.BP_BossHP_C"))
      (UserInterface|Viewport|AddtoViewport _returnvalue 0)
      (Game|SpawnActorfromClass "/Game/_VirusGame/AI/AIOperatingSystem/brain_BP.brain_BP_C" (Math|Transform|MakeTransform (Math|Vector|MakeVector 6.6e+02 1.01e+03 -4.04e+03) (Math|Rotator|MakeRotator 0.0 0.0 -9e+01) "1.000000,1.000000,1.000000") "Undefined" 0 0))
    (:CastFailed
      (Development|PrintString "Hello"))))

(event EventBeginPlay)

(event Collision|EventActorBeginOverlap
  (params (OtherActor :type Actor%20Object%20Reference)))

(event EventTick
  (params (DeltaSeconds :type Float%20%28single-precision%29)))

(fn ConstructionScript)