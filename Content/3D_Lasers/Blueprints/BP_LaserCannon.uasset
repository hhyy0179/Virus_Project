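; BP_LaserCannon is a mouse-aimed laser cannon that previews ten different laser effect Blueprints.
; Each Tick it rotates its Sphere toward the cursor's WorldStatic hit, or toward a far point along the deprojected cursor ray when nothing is hit.
; Left/A and Right/D cycle the selected laser with wraparound.
; Holding left mouse spawns that laser at FirePoint, Tick keeps it aligned to the aim, and release destroys it.
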(event EventTick
  (params (DeltaSeconds :type Float%20%28single-precision%29))
  (bind _returnvalue (Game|GetPlayerController 0))
  (bind _array (Utilities|Array|MakeArray "ObjectTypeQuery1"))
  (bind _sphere (Variables|Default|GetSphere))
  (bind _firepoint (Variables|Default|GetFirePoint))
  (bind (_locationx _locationy) (Game|Player|GetMousePosition _returnvalue))
  (bind _hitresult (Class|PlayerController|GetHitResultUnderCursorforObjects _returnvalue _array true))
  (bind _returnvalue_2 (Transformation|GetWorldLocation _firepoint))
  (bind _returnvalue_3 (Math|Vector2D|MakeVector2D _locationx _locationy))
  (bind (_bblockinghit _binitialoverlap _time _distance _location) (Collision|BreakHitResult _hitresult))
  (bind (_worldposition _worlddirection) (Class|GameplayStatics|DeprojectScreentoWorld _returnvalue _returnvalue_3))
  (if _bblockinghit
    (Transformation|SetWorldRotation _sphere (Math|Rotator|FindLookatRotation _returnvalue_2 _location) false false)
    (else
      (Transformation|SetWorldRotation _sphere (Math|Rotator|FindLookatRotation _returnvalue_2 (+ _worldposition (* _worlddirection 1e+05))) false false)))
  (Utilities|IsValid (stale Input|MouseEvents|LeftMouseButton _returnvalue)
    (:Is%20Valid
      (Transformation|SetActorTransform (stale Input|MouseEvents|LeftMouseButton _returnvalue) (Math|Transform|MakeTransform _returnvalue_2 (Transformation|GetWorldRotation (Variables|Default|GetSphere)))))))

(event Input|MouseEvents|LeftMouseButton
  (params (Key :type Key%20Structure))
  (:Pressed
    (bind _returnvalue (Game|SpawnActorfromClass (Utilities|Array|Get(acopy) (Utilities|Array|MakeArray "/Game/3D_Lasers/Blueprints/BP_Laser_1.BP_Laser_1_C" "/Game/3D_Lasers/Blueprints/BP_Laser_2.BP_Laser_2_C" "/Game/3D_Lasers/Blueprints/BP_Laser_3.BP_Laser_3_C" "/Game/3D_Lasers/Blueprints/BP_Laser_4.BP_Laser_4_C" "/Game/3D_Lasers/Blueprints/BP_Laser_5.BP_Laser_5_C" "/Game/3D_Lasers/Blueprints/BP_Laser_6.BP_Laser_6_C" "/Game/3D_Lasers/Blueprints/BP_Laser_7.BP_Laser_7_C" "/Game/3D_Lasers/Blueprints/BP_Laser_8.BP_Laser_8_C" "/Game/3D_Lasers/Blueprints/BP_Laser_9.BP_Laser_9_C" "/Game/3D_Lasers/Blueprints/BP_Laser_10.BP_Laser_10_C") (Math|Float|Truncate (Variables|Default|GetEffect%20Number))) (Math|Transform|MakeTransform (Transformation|GetWorldLocation (Variables|Default|GetFirePoint)) (Transformation|GetWorldRotation (Variables|Default|GetSphere))) "Undefined" 0 0)))
  (:Released
    (Actor|DestroyActor _returnvalue)))

(event Input|KeyboardEvents|D
  (params (Key :type Key%20Structure))
  (:Pressed
    (if (> (+ 1.0 (Variables|Default|GetEffect%20Number)) (- (Math|Conversions|ToFloat(Integer) (Utilities|Array|Length (Utilities|Array|MakeArray "/Game/3D_Lasers/Blueprints/BP_Laser_1.BP_Laser_1_C" "/Game/3D_Lasers/Blueprints/BP_Laser_2.BP_Laser_2_C" "/Game/3D_Lasers/Blueprints/BP_Laser_3.BP_Laser_3_C" "/Game/3D_Lasers/Blueprints/BP_Laser_4.BP_Laser_4_C" "/Game/3D_Lasers/Blueprints/BP_Laser_5.BP_Laser_5_C" "/Game/3D_Lasers/Blueprints/BP_Laser_6.BP_Laser_6_C" "/Game/3D_Lasers/Blueprints/BP_Laser_7.BP_Laser_7_C" "/Game/3D_Lasers/Blueprints/BP_Laser_8.BP_Laser_8_C" "/Game/3D_Lasers/Blueprints/BP_Laser_9.BP_Laser_9_C" "/Game/3D_Lasers/Blueprints/BP_Laser_10.BP_Laser_10_C"))) 1.0))
      (Variables|Default|SetEffect%20Number 0.0)
      (else
        (Variables|Default|SetEffect%20Number (+ 1.0 (Variables|Default|GetEffect%20Number)))))))

(event Input|KeyboardEvents|Left
  (params (Key :type Key%20Structure))
  (:Pressed
    (if (> 0.0 (- (Variables|Default|GetEffect%20Number) 1.0))
      (Variables|Default|SetEffect%20Number (- (Math|Conversions|ToFloat(Integer) (Utilities|Array|Length (Utilities|Array|MakeArray "/Game/3D_Lasers/Blueprints/BP_Laser_1.BP_Laser_1_C" "/Game/3D_Lasers/Blueprints/BP_Laser_2.BP_Laser_2_C" "/Game/3D_Lasers/Blueprints/BP_Laser_3.BP_Laser_3_C" "/Game/3D_Lasers/Blueprints/BP_Laser_4.BP_Laser_4_C" "/Game/3D_Lasers/Blueprints/BP_Laser_5.BP_Laser_5_C" "/Game/3D_Lasers/Blueprints/BP_Laser_6.BP_Laser_6_C" "/Game/3D_Lasers/Blueprints/BP_Laser_7.BP_Laser_7_C" "/Game/3D_Lasers/Blueprints/BP_Laser_8.BP_Laser_8_C" "/Game/3D_Lasers/Blueprints/BP_Laser_9.BP_Laser_9_C" "/Game/3D_Lasers/Blueprints/BP_Laser_10.BP_Laser_10_C"))) 1.0))
      (else
        (Variables|Default|SetEffect%20Number (- (Variables|Default|GetEffect%20Number) 1.0))))))

(event Input|KeyboardEvents|A
  (params (Key :type Key%20Structure))
  (:Pressed
    (if (> 0.0 (- (Variables|Default|GetEffect%20Number) 1.0))
      (Variables|Default|SetEffect%20Number (- (Math|Conversions|ToFloat(Integer) (Utilities|Array|Length (Utilities|Array|MakeArray "/Game/3D_Lasers/Blueprints/BP_Laser_1.BP_Laser_1_C" "/Game/3D_Lasers/Blueprints/BP_Laser_2.BP_Laser_2_C" "/Game/3D_Lasers/Blueprints/BP_Laser_3.BP_Laser_3_C" "/Game/3D_Lasers/Blueprints/BP_Laser_4.BP_Laser_4_C" "/Game/3D_Lasers/Blueprints/BP_Laser_5.BP_Laser_5_C" "/Game/3D_Lasers/Blueprints/BP_Laser_6.BP_Laser_6_C" "/Game/3D_Lasers/Blueprints/BP_Laser_7.BP_Laser_7_C" "/Game/3D_Lasers/Blueprints/BP_Laser_8.BP_Laser_8_C" "/Game/3D_Lasers/Blueprints/BP_Laser_9.BP_Laser_9_C" "/Game/3D_Lasers/Blueprints/BP_Laser_10.BP_Laser_10_C"))) 1.0))
      (else
        (Variables|Default|SetEffect%20Number (- (Variables|Default|GetEffect%20Number) 1.0))))))

(event Input|KeyboardEvents|Right
  (params (Key :type Key%20Structure))
  (:Pressed
    (if (> (+ 1.0 (Variables|Default|GetEffect%20Number)) (- (Math|Conversions|ToFloat(Integer) (Utilities|Array|Length (Utilities|Array|MakeArray "/Game/3D_Lasers/Blueprints/BP_Laser_1.BP_Laser_1_C" "/Game/3D_Lasers/Blueprints/BP_Laser_2.BP_Laser_2_C" "/Game/3D_Lasers/Blueprints/BP_Laser_3.BP_Laser_3_C" "/Game/3D_Lasers/Blueprints/BP_Laser_4.BP_Laser_4_C" "/Game/3D_Lasers/Blueprints/BP_Laser_5.BP_Laser_5_C" "/Game/3D_Lasers/Blueprints/BP_Laser_6.BP_Laser_6_C" "/Game/3D_Lasers/Blueprints/BP_Laser_7.BP_Laser_7_C" "/Game/3D_Lasers/Blueprints/BP_Laser_8.BP_Laser_8_C" "/Game/3D_Lasers/Blueprints/BP_Laser_9.BP_Laser_9_C" "/Game/3D_Lasers/Blueprints/BP_Laser_10.BP_Laser_10_C"))) 1.0))
      (Variables|Default|SetEffect%20Number 0.0)
      (else
        (Variables|Default|SetEffect%20Number (+ 1.0 (Variables|Default|GetEffect%20Number)))))))

(fn ConstructionScript)